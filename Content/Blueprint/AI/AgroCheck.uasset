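; AgroCheck is a Behavior Tree service that lets AI pawns detect nearby targets to follow.
; Each tick it caches the AI controller, then sphere-traces around the controlled pawn, ignoring all Bp_EnemyGrabber actors.
; A camera-channel line trace tests visibility of each hit.
; Visible actors set the TargetToFollow and TargetLocation blackboard keys, while blocked ones clear TargetToFollow, so the last hit processed wins.
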(event EventTick
  (params (OwnerActor :type Actor%20Object%20Reference) (DeltaSeconds :type Float%20%28single-precision%29))
  ;[1 1 1] Ticked to a rate defined in the Behavior Tree
  ;[1 1 1] Is AI controller ref set?
  (if (!= (Variables|Default|GetAI_Controller_Ref) 0)
    _
    (else
      (bind _asai_controller (Utilities|Casting|CastToAI_Controller OwnerActor))
      (Variables|Default|SetAI_Controller_Ref _asai_controller)))
  (bind _outactors (Actor|GetAllActorsOfClass "/Game/Blueprint/bp_EnemyGrabber.bp_EnemyGrabber_C"))
  (Variables|Default|SetMyLocation (Transformation|GetActorLocation (Pawn|GetControlledPawn (Variables|Default|GetAI_Controller_Ref))))
  ;[1 1 1] Do a Multi Sphere Trace for Objects based on the location of the controlled pawn, and get all the pawns, minus the controlled pawn
  (bind _outhits (Collision|MultiSphereTraceForObjects (Transformation|GetActorLocation (Pawn|GetControlledPawn (Variables|Default|GetAI_Controller_Ref))) (+ (Transformation|GetActorLocation (Pawn|GetControlledPawn (Variables|Default|GetAI_Controller_Ref))) "0, 0,15.000000") 5e+02 (Variables|Default|GetDesiredObjectTypes) false _outactors "None"))
  ;[1 1 1] Figures out if the player was hit
  (bind _array_element (Utilities|Array|ForEachLoopwithBreak _outhits)
    (:LoopBody
      ;[1 1 1] do a visibility trace to see if our AI pawn can see the player pawn.
      (bind _outhit (Collision|LineTraceByChannel (Variables|Default|GetMyLocation) (Transformation|GetActorLocation (.HitActor (Collision|BreakHitResult _array_element))) "TraceTypeQuery2" false _outactors "None"))
      ;[1 1 1] set the appropriate values on the blackboard object for the AI pawn
      (if (== (.HitActor (Collision|BreakHitResult _outhit)) (.HitActor (Collision|BreakHitResult _array_element)))
        (Class|BTFunctionLibrary|SetBlackboardValueasObject (Variables|Default|GetTargetToFollow) (.HitActor (Collision|BreakHitResult _outhit)))
        (AI|BehaviorTree|SetBlackboardValueasVector (Variables|Default|GetTargetLocation) (Transformation|GetActorLocation (.HitActor (Collision|BreakHitResult _outhit))))
        (else
          ;[1 1 1] clear the Target to Follow key on the blackboard
          (Class|BTFunctionLibrary|SetBlackboardValueasObject (Variables|Default|GetTargetToFollow)))))))