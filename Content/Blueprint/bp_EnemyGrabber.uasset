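; Enemy grabber Blueprint that immobilizes the LittleGirl character on contact and toggles a Widget's visibility by proximity.
; Beginning an overlap shows the Widget unless the Grabbed flag is set, and ending an overlap hides it.
; A capsule hit on LittleGirl zeroes her walk speed and jump velocity and prints a debug message.
; This graph never sets Grabbed or restores her movement.
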(event OnComponentHit(CapsuleComponent)
  (params (HitComponent :type Primitive%20Component%20Object%20Reference) (OtherActor :type Actor%20Object%20Reference) (OtherComp :type Primitive%20Component%20Object%20Reference) (NormalImpulse :type Vector :default "0, 0, 0") (Hit :type Hit%20Result%20Structure%20%28by%20ref%29))
  (bind _aslittle_girl (Utilities|Casting|CastToLittleGirl OtherActor))
  (bind _output_get (Variables|/Script/Engine.CharacterMovementComponent|SetMaxWalkSpeed (Variables|/Script/Engine.Character|GetCharacterMovement _aslittle_girl) 0.0))
  (Variables|/Script/Engine.CharacterMovementComponent|SetJumpZVelocity (Variables|/Script/Engine.Character|GetCharacterMovement _aslittle_girl) _output_get)
  (Development|PrintString "Grabbed!"))

(event Collision|EventActorBeginOverlap
  (params (OtherActor :type Actor%20Object%20Reference))
  (if (Variables|Default|GetGrabbed)
    (Rendering|SetVisibility (Variables|Default|GetWidget) false false)
    (else
      (Rendering|SetVisibility (Variables|Default|GetWidget) true false))))

(event Collision|EventActorEndOverlap
  (params (OtherActor :type Actor%20Object%20Reference))
  (Rendering|SetVisibility (Variables|Default|GetWidget) false false))

(fn ConstructionScript)