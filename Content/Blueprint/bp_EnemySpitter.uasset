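; Enemy spitter Blueprint that turns and spits while the player character is within attack range.
; Tick runs SpittandTurn, which first calls AgroCheck to set InRange by comparing player distance to AttackRange.
; In range, a Sequence calls Turning immediately and Spitting after a Delay that paces attacks; out of range, a RetriggerableDelay leads to another range check.
; Turning and Spitting are called but not defined here.
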(event Custom|AgroCheck
  ;[1 1 1] Check if player is within range
  (if (< (Transformation|GetDistanceTo (Game|GetPlayerCharacter 0)) (Variables|Default|GetAttackRange))
    (Variables|Default|SetInRange true)
    (else
      (Variables|Default|SetInRange false))))

(event Custom|Spitt%20and%20Turn
  ;[1 1 1] Spitt and turn when player is within range.
  (CallFunction|AgroCheck)
  (if (Variables|Default|GetInRange)
    (Utilities|FlowControl|Sequence
      (:then_0
        (Class|EnemySpitter|Turning))
      (:then_1
        (Utilities|FlowControl|Delay 1.0)
        (Class|EnemySpitter|Spitting)))
    (else
      (Utilities|FlowControl|RetriggerableDelay 0.2)
      (CallFunction|AgroCheck))))

(event EventBeginPlay)

(event Collision|EventActorBeginOverlap
  (params (OtherActor :type Actor%20Object%20Reference)))

(event EventTick
  (params (DeltaSeconds :type Float%20%28single-precision%29))
  ;[1 1 1] Spitt and turn when player is within range.
  (CallFunction|SpittandTurn))

(fn ConstructionScript)