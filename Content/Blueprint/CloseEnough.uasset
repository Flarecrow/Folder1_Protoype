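; CloseEnough is a behavior tree decorator that gates a branch on the distance between an AI's pawn and its follow target.
; It casts the owner to AI_Controller, caches it, and reads the target actor from the TargetToFollow blackboard key.
; Despite the name, the condition passes when the straight-line distance is at or beyond AcceptableDistance, so it is true while the pawn is not yet close enough.
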(fn PerformConditionCheck
  (params (OwnerActor :type Actor%20Object%20Reference))
  (bind _asai_controller (Utilities|Casting|CastToAI_Controller OwnerActor))
  (Variables|Default|SetAI_Controller_Ref _asai_controller)
  (return (>= (Math|Vector|VectorLength (- (Transformation|GetActorLocation (AI|BehaviorTree|GetBlackboardValueasActor (Variables|Default|GetTargetToFollow))) (Transformation|GetActorLocation (Pawn|GetControlledPawn (Variables|Default|GetAI_Controller_Ref))))) (Variables|Default|GetAcceptableDistance))))